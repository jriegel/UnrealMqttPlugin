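; BP_MQTT_Test_Actor is a test actor that exercises MQTT messaging through a client configured for a broker on localhost.
; BeginPlay enables player input, creates and stores the client, binds a message handler and subscribes with an empty topic, with no explicit connect call.
; Pressing E publishes a fixed test message to the "test" topic, and the handler prints any received message on screen in green.
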(event Custom|OnMqttMessage
  (params (message :type Mqtt%20Message%20Structure))
  (Development|PrintString (.message message) true true "(R=0.489789,G=1.000000,B=0.171030,A=1.000000)"))

(event EventBeginPlay
  (Input|EnableInput (Game|GetPlayerController 0))
  (bind _returnvalue (Class|MqttUtilitiesBPL|CreateMqttClient (Utilities|Struct|MakeMqttClientConfig "localhost" 0 "UeTest" -1)))
  (bind _output_get (Variables|Default|SetMqttClient _returnvalue))
  (Class|MqttClientInterface|SetonMessageHandler _output_get (delegate Custom|OnMqttMessage))
  (Class|MqttClientInterface|Subscribe _output_get))

(event EventTick
  (params (DeltaSeconds :type Float%20%28single-precision%29)))

(event Input|KeyboardEvents|E
  (params (Key :type Key%20Structure :default "None"))
  (:Pressed
    (Class|MqttClientInterface|Publish (Variables|Default|GetMqttClient) (Utilities|Struct|MakeMqttMessage "test" "test" false))))

(fn ConstructionScript)